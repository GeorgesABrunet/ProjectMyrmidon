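; Robot player character, extending a parent character with its own mantle, get-up and ragdoll recovery setup, exposing grapple and wingsuit components through interface getters.
; BeginPlay creates the health HUD and registers with GS_Test's player list, which spectate events cycle through.
; Tick widens camera FOV during fast airborne or gliding movement when reeling or moving vertically, easing back otherwise.
; A smoothed, collision-traced follow-camera routine exists but is unwired.
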(event Custom|SpectateNextPlayer
  (bind _as_gs_test (Variables|Default|GetAs%20GS%20Test))
  (bind _playerlist (Variables|/Game/GMs/GS_Test.GS_Test_C|GetPlayerList _as_gs_test))
  ;[1 1 1] spectator bullshit
  (if (== (+ (Variables|Default|GetSpectatingPlayer) 1) (Utilities|Array|Length _playerlist))
    (Variables|Default|SetSpectatingPlayer 0)
    (else
      (Variables|Default|SetSpectatingPlayer (+ (Variables|Default|GetSpectatingPlayer) 1))))
  (Game|Player|SetViewTargetwithBlend (Game|GetPlayerController 0) (Utilities|Array|Get(acopy) _playerlist (Variables|Default|GetSpectatingPlayer)) 0.0 "VTBlend_Linear" 0.0 false))

(event Custom|SpectatePreviousPlayer
  (bind _as_gs_test (Variables|Default|GetAs%20GS%20Test))
  (bind _playerlist (Variables|/Game/GMs/GS_Test.GS_Test_C|GetPlayerList _as_gs_test))
  ;[1 1 1] spectator bullshit
  (if (== (- (Variables|Default|GetSpectatingPlayer) 1) -1)
    (Variables|Default|SetSpectatingPlayer (- (Utilities|Array|Length _playerlist) 1))
    (else
      (Variables|Default|SetSpectatingPlayer (- (Variables|Default|GetSpectatingPlayer) 1))))
  (Game|Player|SetViewTargetwithBlend (Game|GetPlayerController 0) (Utilities|Array|Get(acopy) _playerlist (Variables|Default|GetSpectatingPlayer)) 0.0 "VTBlend_Linear" 0.0 false))

(event EventBeginPlay
  (|CallParentFunction)
  (CallFunction|SetUpBeginPlay))

(event Collision|EventActorBeginOverlap
  (params (OtherActor :type Actor%20Object%20Reference)))

(event EventTick
  (params (DeltaSeconds :type Float%20%28single-precision%29))
  (|CallParentFunction DeltaSeconds)
  (CallFunction|AffectFOV)
  (Camera|SetFieldOfView (Variables|Default|GetCamera) (Variables|Default|GetThirdPersonFOV)))

(fn ConstructionScript
  (|CallParentFunction))

(fn SetUpBeginPlay
  (Utilities|FlowControl|Sequence
    (:then_0
      (bind _asplayer_controller (Utilities|Casting|CastToPlayerController (Pawn|GetController)))
      (bind _returnvalue (UserInterface|CreateWidget "/Game/UI/HUD_Player.HUD_Player_C" _asplayer_controller))
      (bind _output_get (Variables|Default|SetHUD _returnvalue))
      (UserInterface|Viewport|AddtoPlayerScreen _output_get)
      (bind _output_get_2 (Variables|/Game/UI/HUD_Player.HUD_Player_C|SetMaxHealth (Variables|Default|GetHUD) 1e+02))
      (Variables|/Game/UI/HUD_Player.HUD_Player_C|SetCurrentHealth (Variables|Default|GetHUD) _output_get_2))
    (:then_1
      (bind _asgs_test (Utilities|Casting|CastToGS_Test (Game|GetGameState)))
      (bind _output_get_3 (Variables|Default|SetAs%20GS%20Test _asgs_test))
      (Default|AddPlayertoList _output_get_3 self))))

(fn RagdollEnd
  (bind _mesh (Variables|Character|GetMesh))
  (|CallParentFunction)
  (Transformation|SetRelativeLocationAndRotation _mesh "0, 0,-46.000000" "0,270.000000, 0" false false)
  (Transformation|AttachComponentToComponent _mesh (Variables|Default|GetCapsuleComponent) "None" "KeepRelative" "KeepRelative" "KeepRelative" true))

(fn GetMantleAsset
  (params (MantleType :type MantleType%20Enum :default "NewEnumerator1"))
  (switch Utilities|FlowControl|Switch|SwitchonMantleType MantleType
    (:NewEnumerator1
      _)
    (:NewEnumerator0
      (return (Variables|Default|GetMantle_1m_Default)))
    (:NewEnumerator2
      _))
  (return (Variables|Default|GetMantle_2m_Default)))

(fn GetGetUpAnimation
  (params (RagdollFaceUp :type Boolean))
  (if RagdollFaceUp
    (return (Variables|Default|GetGetUpBack_Default))
    (else
      (return (Variables|Default|GetGetUpFront_Default)))))

(fn AffectFOV
  (bind _verticalmotion (Variables|Default|GetVerticalMotion))
  (|CallParentFunction)
  (switch Utilities|FlowControl|Switch|SwitchonALS_MovementState (Variables|Default|GetMovementState)
    (:NewEnumerator2
      _)
    (:NewEnumerator6
      _))
  (if (and (or (Variables|/Game/BPs/ActorCmpnts/Grapple/GrappleComponent.GrappleComponent_C|GetbIsReeling (Variables|Default|GetGrappleComponent)) _verticalmotion) (> (Math|Vector|VectorLength (Transformation|GetVelocity)) 6e+02))
    (Variables|Default|SetThirdPersonFOV (Math|Float|Clamp(Float) (+ (Variables|Default|GetThirdPersonFOV) 0.08 (* (Math|Conversions|ToFloat(Boolean) _verticalmotion) 0.5)) 9e+01 1.2e+02))
    (else
      (Variables|Default|SetThirdPersonFOV (Math|Float|Clamp(Float) (- (Variables|Default|GetThirdPersonFOV) 0.32) 9e+01 1.2e+02)))))

(fn CameraUpdates
  (bind _self self)
  (Utilities|FlowControl|Sequence
    (:then_0
      ;[1 1 1] Step 1: Get Camera Parameters
      (bind _returnvalue (Class|BPICameraSys|BPIGetCameraTarget(Message) _self))
      (LocalVariables|SetPivotTarget _returnvalue)
      (bind _armlength (Class|BPICameraSys|BPIGetCameraParameters(Message) _self))
      (Variables|Default|SetCurrentArmLength _armlength))
    (:then_1
      ;[1 1 1] Step 2: Interpolate Camera Rotation
      (Variables|Default|SetTargetCameraRot (Math|Interpolation|RInterpTo (Variables|/Script/Engine.SceneComponent|GetRelativeRotation (Variables|Default|GetCamera)) (Pawn|GetControlRotation :!class /Script/Engine.Pawn) (Utilities|Time|GetWorldDeltaSeconds) 6.0)))
    (:then_2
      ;[1 1 1] Step 3: Calculate Smoothed Pivot Target
      (LocalVariables|SetSmoothedPivotTarget (Math|Transform|MakeTransform (CallFunction|CalculateAxisIndependentLag (.location (LocalVariables|GetSmoothedPivotTarget)) (.location (LocalVariables|GetPivotTarget)) (Variables|Default|GetTargetCameraRot) (* "1.000000,1.000000,1.000000" (LocalVariables|GetLagSpeeds))) (.rotation (LocalVariables|GetPivotTarget)))))
    (:then_3
      ;[1 1 1] Step 4: Set Target Camera Location
      (LocalVariables|SetPivotLocation (+ (.location (LocalVariables|GetSmoothedPivotTarget)) (* (Math|Vector|GetForwardVector (.rotation (LocalVariables|GetSmoothedPivotTarget))) (* (Variables|Default|GetCurrentArmLength) -1.0)) (* (Math|Vector|GetUpVector (.rotation (LocalVariables|GetSmoothedPivotTarget))) (* (Variables|Default|GetCurrentArmLength) 0.3)) ""))
      (LocalVariables|SetTargetCameraLocation (LocalVariables|GetPivotLocation)))
    (:then_4
      ;[1 1 1] Step 5: Trace between Target  & Camera for Collisions and Adjust Camera Location
      (bind _outhit (Collision|SphereTraceForObjects (.location (LocalVariables|GetPivotTarget)) (LocalVariables|GetTargetCameraLocation) 1e+01 (Utilities|Array|MakeArray "ObjectTypeQuery1" "ObjectTypeQuery2" "ObjectTypeQuery4") false 0 "None"))
      (if (and (.bBlockingHit (Collision|BreakHitResult _outhit)) (not (.bInitialOverlap (Collision|BreakHitResult _outhit))))
        (LocalVariables|SetTargetCameraLocation (+ (- (.Location (Collision|BreakHitResult _outhit)) (.TraceEnd (Collision|BreakHitResult _outhit))) (LocalVariables|GetTargetCameraLocation)))))
    (:then_5
      ;[1 1 1] Return Camera Behavior
      (return (LocalVariables|GetPivotLocation) (Variables|Default|GetTargetCameraRot)))))

(fn CalculateAxisIndependentLag
  (params (CurrentLocation :type Vector) (TargetLocation :type Vector) (CameraRotation :type Rotator) (LagSpeeds :type Vector))
  (bind _returnvalue (Utilities|Time|GetWorldDeltaSeconds))
  (bind (_x _y _z) (Math|Vector|BreakVector LagSpeeds))
  (LocalVariables|SetCameraRotationAngles (Math|Rotator|MakeRotator 0.0 0.0 (.yaw CameraRotation)))
  (return (Math|Vector|RotateVector (Math|Vector|MakeVector (Math|Interpolation|FInterpTo (.x (Math|Vector|UnrotateVector CurrentLocation (LocalVariables|GetCameraRotationAngles))) (.x (Math|Vector|UnrotateVector TargetLocation (LocalVariables|GetCameraRotationAngles))) _returnvalue _x) (Math|Interpolation|FInterpTo (.y (Math|Vector|UnrotateVector CurrentLocation (LocalVariables|GetCameraRotationAngles))) (.y (Math|Vector|UnrotateVector TargetLocation (LocalVariables|GetCameraRotationAngles))) _returnvalue _y) (Math|Interpolation|FInterpTo (.z (Math|Vector|UnrotateVector CurrentLocation (LocalVariables|GetCameraRotationAngles))) (.z (Math|Vector|UnrotateVector TargetLocation (LocalVariables|GetCameraRotationAngles))) _returnvalue _z)) (LocalVariables|GetCameraRotationAngles))))

(fn OnRepWingsuitComponent)

(fn BPIGetGlidingComponent
  (return 0))

(fn BPIGetGrapplingComponent
  (return (Variables|Default|GetGrappleComponent)))

(fn BPIGetWingsuitComponent
  (return (Variables|Default|GetWingsuitComponent)))