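; Base projectile Blueprint with a collision sphere, mesh and explosion effect, apparently unfinished.
; Sphere hit and overlap events print debug messages and call OnHitEvent, which passes blocking or initial-overlap impacts to DetermineImpact.
; DetermineImpact runs a debug-drawn multi-sphere trace around the impact point, but its loop over the results is empty.
; DestroyProjectile hides the mesh and activates the explosion without destroying the actor, and is not called within this Blueprint.
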(event OnComponentHit(Sphere)
  (params (HitComponent :type Primitive%20Component%20Object%20Reference) (OtherActor :type Actor%20Object%20Reference) (OtherComp :type Primitive%20Component%20Object%20Reference) (NormalImpulse :type Vector :default "0, 0, 0") (Hit :type Hit%20Result%20Structure%20%28by%20ref%29))
  (Development|PrintString (Utilities|String|Append "Hit Event -- " (Utilities|GetDisplayName self) " has hit: " (Utilities|GetDisplayName OtherActor)))
  (CallFunction|OnHitEvent Hit))

(event OnComponentBeginOverlap(Sphere)
  (params (OverlappedComponent :type Primitive%20Component%20Object%20Reference) (OtherActor :type Actor%20Object%20Reference) (OtherComp :type Primitive%20Component%20Object%20Reference) (OtherBodyIndex :type Integer) (bFromSweep :type Boolean) (SweepResult :type Hit%20Result%20Structure%20%28by%20ref%29))
  (Development|PrintString (Utilities|String|Append "Hit Event -- " (Utilities|GetDisplayName self) " has hit: " (Utilities|GetDisplayName 0)))
  (CallFunction|OnHitEvent SweepResult))

(event EventBeginPlay)

(event Collision|EventActorBeginOverlap
  (params (OtherActor :type Actor%20Object%20Reference)))

(event EventTick
  (params (DeltaSeconds :type Float%20%28single-precision%29)))

(fn ConstructionScript)

(fn OnHitEvent
  (params (Hit :type Hit%20Result%20Structure))
  (bind (_bblockinghit _binitialoverlap _time _distance _location _impactpoint) (Collision|BreakHitResult Hit))
  (if (or _bblockinghit _binitialoverlap)
    (CallFunction|DetermineImpact _impactpoint)))

(fn DetermineImpact
  (params (Location :type Vector))
  (bind _outhits (Collision|MultiSphereTraceForObjects Location (+ Location "0,0.000000,0.010000") 1e+02 (Utilities|Array|MakeArray "ObjectTypeQuery1" "ObjectTypeQuery2" "ObjectTypeQuery3" "ObjectTypeQuery4") false 0 "ForDuration"))
  (for _array_element _outhits
    _))

(fn DestroyProjectile
  (Rendering|SetVisibility (Variables|Default|GetStaticMesh) false false)
  (Components|Activation|Activate (Variables|Default|GetExplosionFX) true))