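; Player controller that links possession to the custom camera system and provides a debug level reset.
; On possess, it casts the camera manager to BP_PlayerCameraSys and passes it the new pawn.
; The DebugReset input reopens the current level by name.
; Its camera interface functions for parameters and target are empty stubs returning default values.
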(event EventPossess
  (params (PossessedPawn :type Pawn%20Object%20Reference))
  (bind _asbp_player_camera_sys (Utilities|Casting|CastToBP_PlayerCameraSys (Variables|Default|GetPlayerCameraManager)))
  (Default|OnPossess _asbp_player_camera_sys PossessedPawn))

(event Input|ActionEvents|InputActionDebugReset
  (params (Key :type Key%20Structure :default "None"))
  (:Pressed
    (bind _returnvalue (Game|GetCurrentLevelName true))
    (Game|OpenLevel(byName) (Utilities|String|StringToName _returnvalue))))

(fn ConstructionScript)

(fn BPIGetCameraParameters
  (return 0.0 0.0))

(fn BPIGetCameraTarget
  (return ""))