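; Player camera manager that overrides BlueprintUpdateCamera to drive a third-person follow camera for the possessed pawn.
; It gets pivot, arm length and FOV from the pawn through interface messages, then smooths rotation toward control rotation.
; The pivot follows with per-axis lag in camera-yaw space, and the camera sits behind and slightly above it.
; A sphere trace from the unsmoothed pivot pulls the camera in on collisions.
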(event Custom|OnPossess
  (params (NewPawn :type Pawn%20Object%20Reference))
  (Variables|Default|SetControlledPawn NewPawn))

(event EventBeginPlay)

(event Collision|EventActorBeginOverlap
  (params (OtherActor :type Actor%20Object%20Reference)))

(event EventTick
  (params (DeltaSeconds :type Float%20%28single-precision%29)))

(fn ConstructionScript)

(fn CustomCameraBehavior
  (bind _controlledpawn (Variables|Default|GetControlledPawn))
  (Utilities|FlowControl|Sequence
    (:then_0
      ;[1 1 1] Step 1: Get Camera Parameters
      (bind _returnvalue (Class|BPICameraSys|BPIGetCameraTarget(Message) _controlledpawn))
      (LocalVariables|SetPivotTarget _returnvalue)
      (bind (_armlength _fov) (Class|BPICameraSys|BPIGetCameraParameters(Message) _controlledpawn))
      (Variables|Default|SetCurrentArmLength _armlength)
      (LocalVariables|SetNewFOV _fov))
    (:then_1
      ;[1 1 1] Step 2: Interpolate Camera Rotation
      (Variables|Default|SetTargetCameraRotation (Math|Interpolation|RInterpTo (Camera|GetCameraRotation) (Pawn|GetControlRotation (Game|Player|GetOwningPlayerController) :!class /Script/Engine.Controller) (Utilities|Time|GetWorldDeltaSeconds) 8.0)))
    (:then_2
      ;[1 1 1] Step 3: Calculate Smoothed Pivot Target
      (Variables|Default|SetSmoothedPivotTarget (Math|Transform|MakeTransform (CallFunction|CalculateAxisIndependentLag (.location (Variables|Default|GetSmoothedPivotTarget)) (.location (LocalVariables|GetPivotTarget)) (Variables|Default|GetTargetCameraRotation) "15.000000,15.000000,15.000000") (.rotation (LocalVariables|GetPivotTarget)))))
    (:then_3
      ;[1 1 1] Step 4: Set Target Camera Location
      (Variables|Default|SetTargetCameraLocation (+ (.location (Variables|Default|GetSmoothedPivotTarget)) (* (Math|Vector|GetForwardVector (Variables|Default|GetTargetCameraRotation)) (* (Variables|Default|GetCurrentArmLength) -1.0)) (* (Math|Vector|GetUpVector (Variables|Default|GetTargetCameraRotation)) (* (Variables|Default|GetCurrentArmLength) 0.2)))))
    (:then_4
      ;[1 1 1] Step 5: Trace between Target  & Camera for Collisions and Adjust Camera Location
      (bind _outhit (Collision|SphereTraceByChannel (.location (LocalVariables|GetPivotTarget)) (Variables|Default|GetTargetCameraLocation) 1e+01 "TraceTypeQuery1" false 0 "None"))
      (if (and (.bBlockingHit (Collision|BreakHitResult _outhit)) (not (.bInitialOverlap (Collision|BreakHitResult _outhit))))
        (Variables|Default|SetTargetCameraLocation (+ (- (.Location (Collision|BreakHitResult _outhit)) (.TraceEnd (Collision|BreakHitResult _outhit))) (Variables|Default|GetTargetCameraLocation)))))
    (:then_5
      ;[1 1 1] Return Camera Behavior
      (return (Variables|Default|GetTargetCameraLocation) (Variables|Default|GetTargetCameraRotation) (LocalVariables|GetNewFOV)))))

(fn BlueprintUpdateCamera
  (params (CameraTarget :type Actor%20Object%20Reference))
  (bind (_location _rotation _fov) (CallFunction|CustomCameraBehavior))
  (return _location _rotation _fov true))

(fn CalculateAxisIndependentLag
  (params (CurrentLocation :type Vector) (TargetLocation :type Vector) (CameraRotation :type Rotator) (LagSpeeds :type Vector))
  (bind _returnvalue (Utilities|Time|GetWorldDeltaSeconds))
  (bind (_x _y _z) (Math|Vector|BreakVector LagSpeeds))
  (LocalVariables|SetCameraRotationAngles (Math|Rotator|MakeRotator 0.0 0.0 (.yaw CameraRotation)))
  (return (Math|Vector|RotateVector (Math|Vector|MakeVector (Math|Interpolation|FInterpTo (.x (Math|Vector|UnrotateVector CurrentLocation (LocalVariables|GetCameraRotationAngles))) (.x (Math|Vector|UnrotateVector TargetLocation (LocalVariables|GetCameraRotationAngles))) _returnvalue _x) (Math|Interpolation|FInterpTo (.y (Math|Vector|UnrotateVector CurrentLocation (LocalVariables|GetCameraRotationAngles))) (.y (Math|Vector|UnrotateVector TargetLocation (LocalVariables|GetCameraRotationAngles))) _returnvalue _y) (Math|Interpolation|FInterpTo (.z (Math|Vector|UnrotateVector CurrentLocation (LocalVariables|GetCameraRotationAngles))) (.z (Math|Vector|UnrotateVector TargetLocation (LocalVariables|GetCameraRotationAngles))) _returnvalue _z)) (LocalVariables|GetCameraRotationAngles))))

(fn BPIGetCameraParameters
  (return 0.0 0.0))

(fn BPIGetCameraTarget
  (return ""))