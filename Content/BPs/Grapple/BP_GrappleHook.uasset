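; Grapple hook actor that reports a successful hook hit to a grapple component.
; On a hit within a maximum range of the character, it records the success, passes the location to the component and changes the grapple state through an interface message.
; A one-shot timer started at BeginPlay backs an auto-destruct event that removes the hook unless a successful hit was recorded.
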(event Custom|AutoDestruct
  (if (Variables|Default|GetbHitSuccess)
    (Utilities|Time|ClearandInvalidateTimerbyHandle (Variables|Default|GetAutoDestructHandle))
    (else
      (Utilities|Time|ClearandInvalidateTimerbyHandle (Variables|Default|GetAutoDestructHandle))
      (Actor|DestroyActor))))

(event EventBeginPlay
  (bind _returnvalue (Utilities|Time|SetTimerbyEvent (EventDispatchers|CreateEvent :!event Custom|AutoDestruct) 5.0))
  (Variables|Default|SetAutoDestructHandle _returnvalue))

(event Collision|EventHit
  (params (MyComp :type Primitive%20Component%20Object%20Reference) (Other :type Actor%20Object%20Reference) (OtherComp :type Primitive%20Component%20Object%20Reference) (bSelfMoved :type Boolean) (HitLocation :type Vector :default "0, 0, 0") (HitNormal :type Vector :default "0, 0, 0") (NormalImpulse :type Vector :default "0, 0, 0") (Hit :type Hit%20Result%20Structure%20%28by%20ref%29))
  (CallFunction|OnHitEvent HitLocation))

(fn ConstructionScript)

(fn OnHitEvent
  (params (HitLocation :type Vector))
  (bind _grapplecomponent (Variables|Default|GetGrappleComponent))
  (if (<= (Math|Vector|VectorLength (- (Transformation|GetActorLocation (Variables|Default|GetCharacter)) HitLocation)) 1e+04)
    (bind _output_get (Variables|Default|SetHitLocation HitLocation))
    (Variables|Default|SetbHitSuccess true)
    (Development|PrintString (Utilities|String|Append "Grapple Hit Location:  " (Utilities|String|ToString(Vector) _output_get)) true false "(R=1.000000,G=0.000000,B=0.007579,A=1.000000)")
    (Variables|/Game/BPs/Grapple/GrappleComponent.GrappleComponent_C|SetGrappleLocation _grapplecomponent _output_get)
    (Class|BPIGrappleInterface|BPISetGrappleState(Message) _grapplecomponent "NewEnumerator1")))