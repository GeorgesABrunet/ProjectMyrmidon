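; Grapple hook projectile that plays a randomly pitched shot sound and self-destructs when it strays too far from its owner, checked on a looping timer.
; On hit, it plays an impact sound, then either attaches to an in-range, non-owner actor or destroys itself.
; A successful hit starts grappling on the owner's component, fetched through an interface.
; Without owner authority, it handles the hit locally and also calls ActorHitEvent to repeat that logic.
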(event Custom|NetworkAutoDestruct
  ;[1 1 1] Multicast call to destroy actor
  (Actor|DestroyActor))

(event Custom|ActorHitEvent
  ;[1 1 1] ActorHitEvent
  (CallFunction|OnHitEventLocal))

(event Custom|ShotSounds
  (bind _shootaudio (Variables|Default|GetShootAudio))
  (Audio|Components|Audio|SetSound _shootaudio (Variables|Default|GetGrappleSound))
  (Audio|Components|Audio|SetPitchMultiplier _shootaudio (Math|Random|RandomFloatinRange 0.4 1.0))
  (Components|Activation|Activate _shootaudio true))

(event Custom|CheckAutoDestruct
  ;[1 1 1] Multicast call to destroy actor
  (if (> (Math|Vector|Distance(Vector) (Transformation|GetActorLocation) (Transformation|GetActorLocation (Components|GetOwner))) 1.5e+04)
    (Utilities|Time|ClearandInvalidateTimerbyHandle (Variables|Default|GetNetworkAutoDestructHandle))
    (CallFunction|NetworkAutoDestruct)))

(event EventBeginPlay
  ;[1 1 1] Activate sound for shot, update to destroy actor if beyond reasonable distance by checking 15 times per second
  (CallFunction|ShotSounds)
  (bind _returnvalue (Utilities|Time|SetTimerbyEvent (EventDispatchers|CreateEvent :!event Custom|CheckAutoDestruct) 0.06667 true))
  (Variables|Default|SetNetworkAutoDestructHandle _returnvalue))

(event Collision|EventHit
  (params (MyComp :type Primitive%20Component%20Object%20Reference) (Other :type Actor%20Object%20Reference) (OtherComp :type Primitive%20Component%20Object%20Reference) (bSelfMoved :type Boolean) (HitLocation :type Vector :default "0, 0, 0") (HitNormal :type Vector :default "0, 0, 0") (NormalImpulse :type Vector :default "0, 0, 0") (Hit :type Hit%20Result%20Structure%20%28by%20ref%29))
  ;[1 1 1] ActorHitEvent
  (CallFunction|ImpactSound)
  (Variables|Default|SetHitActor Other)
  (Variables|Default|SetHitLocation HitLocation)
  (if (Ability|HasAuthority (Components|GetOwner))
    (CallFunction|OnHitEventLocal)
    (else
      (CallFunction|OnHitEventLocal)
      (CallFunction|ActorHitEvent))))

(fn ConstructionScript)

(fn OnHitEvent
  (params (HitLocation :type Vector) (ActorHit :type Actor%20Object%20Reference))
  (bind _returnvalue (Components|GetOwner))
  (bind _returnvalue_2 (Transformation|GetActorLocation _returnvalue))
  (bind _returnvalue_3 (- _returnvalue_2 HitLocation))
  (bind _returnvalue_4 (Math|Vector|VectorLength _returnvalue_3))
  (if (and (<= _returnvalue_4 1e+04) (!= ActorHit _returnvalue))
    (Variables|Default|SetbHitSuccess true)
    (Variables|/Script/CableComponent.CableComponent|SetCableLength (Variables|Default|GetCable) _returnvalue_4)
    (Development|PrintString (Utilities|String|Append (Utilities|GetDisplayName self) "Grapple Hit Location: " (Utilities|String|ToString(Vector) HitLocation) " --- Hit: " (Utilities|GetDisplayName ActorHit)) false true "(R=1.000000,G=0.000000,B=0.007579,A=1.000000)")
    (Transformation|AttachActorToActor ActorHit "None" "KeepWorld" "KeepWorld" "KeepWorld" true)
    (bind _grapplingcomponent (Class|BPIActiveComponents|BPIGetGrapplingComponent(Message) (Components|GetOwner)))
    (Default|StartGrappling _grapplingcomponent)
    (return HitLocation ActorHit)
    (else
      (Actor|DestroyActor))))

(fn ImpactSound
  (Audio|PlaySoundatLocation (Variables|Default|GetImpactSoundCue) (Transformation|GetActorLocation) "0, 0, 0" 0.4 (Math|Random|RandomFloatinRange 0.4 1.0) 0.0 0 0 0 0))

(fn OnHitEventLocal
  (bind _returnvalue (Components|GetOwner))
  (bind _hitactor (Variables|Default|GetHitActor)
    (:then
      (if (and (<= (Math|Vector|Distance(Vector) (Variables|Default|GetHitLocation) (Transformation|GetActorLocation _returnvalue)) 1e+04) (!= _hitactor _returnvalue))
        (Variables|Default|SetbHitSuccess true)
        (Transformation|AttachActorToActor (Variables|Default|GetHitActor) "None" "KeepWorld" "KeepWorld" "KeepWorld" true)
        (bind _grapplingcomponent (Class|BPIActiveComponents|BPIGetGrapplingComponent(Message) (Components|GetOwner)))
        (Utilities|IsValid _grapplingcomponent
          (:Is%20Valid
            (Default|StartGrappling _grapplingcomponent)))
        (else
          (Actor|DestroyActor))))
    (:else)))