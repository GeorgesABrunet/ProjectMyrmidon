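; BP_RobotChar is a robot character Blueprint that adds gliding and grappling to a parent character with mantle and ragdoll support.
; BeginPlay creates the health HUD and attaches the glider mesh to a socket for the GlidingComponent.
; Tick widens third-person FOV while airborne or gliding during grapple reeling or vertical motion, otherwise narrowing it in those states.
; Overrides supply mantle and get-up assets and reattach the mesh after ragdoll, while interface functions expose both traversal components.
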(event EventBeginPlay
  (|CallParentFunction)
  (CallFunction|SetUpBeginPlay))

(event Collision|EventActorBeginOverlap
  (params (OtherActor :type Actor%20Object%20Reference)))

(event EventTick
  (params (DeltaSeconds :type Float%20%28single-precision%29))
  (|CallParentFunction DeltaSeconds)
  (CallFunction|AffectFOV))

(fn ConstructionScript
  (|CallParentFunction))

(fn SetUpBeginPlay
  (bind _glider (Variables|Default|GetGlider))
  (bind _returnvalue (UserInterface|CreateWidget "/Game/BPs/HUD.HUD_C" (Game|GetPlayerController 0)))
  (bind _output_get (Variables|Default|SetHUD _returnvalue))
  (UserInterface|Viewport|AddtoPlayerScreen _output_get)
  (bind _output_get_2 (Variables|/Game/BPs/HUD.HUD_C|SetMaxHealth (Variables|Default|GetHUD) 1e+02))
  (Variables|/Game/BPs/HUD.HUD_C|SetCurrentHealth (Variables|Default|GetHUD) _output_get_2)
  ;[1 1 1] Gliding Component parameters
  (Transformation|AttachComponentToComponent _glider (Variables|Character|GetMesh) "glider01" "SnapToTarget" "SnapToTarget" "KeepRelative" true)
  (Variables|/Game/BPs/Gliding/GlidingComponent.GlidingComponent_C|SetGliderMesh (Variables|Default|GetGlidingComponent) _glider))

(fn RagdollEnd
  (bind _mesh (Variables|Character|GetMesh))
  (|CallParentFunction)
  (Transformation|SetRelativeLocationAndRotation _mesh "0, 0,-46.000000" "0,270.000000, 0" false false)
  (Transformation|AttachComponentToComponent _mesh (Variables|Default|GetCapsuleComponent) "None" "KeepRelative" "KeepRelative" "KeepRelative" true))

(fn GetMantleAsset
  (params (MantleType :type MantleType%20Enum :default "NewEnumerator1"))
  (switch Utilities|FlowControl|Switch|SwitchonMantleType MantleType
    (:NewEnumerator1
      _)
    (:NewEnumerator0
      (return (Variables|Default|GetMantle_1m_Default)))
    (:NewEnumerator2
      _))
  (return (Variables|Default|GetMantle_2m_Default)))

(fn GetGetUpAnimation
  (params (RagdollFaceUp :type Boolean))
  (if RagdollFaceUp
    (return (Variables|Default|GetGetUpBack_Default))
    (else
      (return (Variables|Default|GetGetUpFront_Default)))))

(fn AffectFOV
  (|CallParentFunction)
  (switch Utilities|FlowControl|Switch|SwitchonALS_MovementState (Variables|Default|GetMovementState)
    (:NewEnumerator2
      _)
    (:NewEnumerator6
      _))
  (if (or (Variables|/Game/BPs/Grapple/GrappleComponent.GrappleComponent_C|GetbIsReeling (Variables|Default|GetGrappleComponent)) (Variables|Default|GetVerticalMotion))
    (Variables|Default|SetThirdPersonFOV (Math|Float|Clamp(Float) (+ (Variables|Default|GetThirdPersonFOV) 0.08 (* 0.0 0.5)) 9e+01 1.2e+02))
    (else
      (Variables|Default|SetThirdPersonFOV (Math|Float|Clamp(Float) (- (Variables|Default|GetThirdPersonFOV) 0.16) 9e+01 1.2e+02)))))

(fn BPIGetGlidingComponent
  (return (Variables|Default|GetGlidingComponent)))

(fn BPIGetGrapplingComponent
  (return (Variables|Default|GetGrappleComponent)))