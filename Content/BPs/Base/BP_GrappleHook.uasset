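; Grapple hook actor that reports a successful hit to BP_Player so the player can grapple to that point.
; On hit, it checks the distance from the player's GrappleBow, and within range sets HitSuccess, stores the GrappleLocation on the player and changes the player's action state.
; A one-shot timer started on BeginPlay drives AutoDestruct, which destroys the hook unless a hit has succeeded.
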(event Custom|AutoDestruct
  (if (Variables|Default|GetbHitSuccess)
    (Utilities|Time|ClearandInvalidateTimerbyHandle (Variables|Default|GetAutoDestructHandle))
    (else
      (Utilities|Time|ClearandInvalidateTimerbyHandle (Variables|Default|GetAutoDestructHandle))
      (Actor|DestroyActor))))

(event EventBeginPlay
  (bind _returnvalue (Utilities|Time|SetTimerbyEvent (EventDispatchers|CreateEvent :!event Custom|AutoDestruct) 5.0))
  (Variables|Default|SetAutoDestructHandle _returnvalue))

(event Collision|EventHit
  (params (MyComp :type Primitive%20Component%20Object%20Reference) (Other :type Actor%20Object%20Reference) (OtherComp :type Primitive%20Component%20Object%20Reference) (bSelfMoved :type Boolean) (HitLocation :type Vector :default "0, 0, 0") (HitNormal :type Vector :default "0, 0, 0") (NormalImpulse :type Vector :default "0, 0, 0") (Hit :type Hit%20Result%20Structure%20%28by%20ref%29))
  (Development|PrintString (Utilities|String|Append (Utilities|GetDisplayName Other) " --- " (Utilities|GetDisplayName OtherComp)) false)
  (bind _asbp_player (Utilities|Casting|CastToBP_Player (Game|GetPlayerCharacter 0)))
  (if (<= (Math|Vector|VectorLength (- HitLocation (Transformation|GetWorldLocation (Variables|/Game/BPs/Base/BP_BaseCharacter.BP_BaseCharacter_C|GetGrappleBow _asbp_player)))) 1e+04)
    (Variables|Default|SetbHitSuccess true)
    (Variables|/Game/BPs/Base/BP_BaseCharacter.BP_BaseCharacter_C|SetGrappleLocation _asbp_player HitLocation)
    (Default|OnActionStateChanged _asbp_player "NewEnumerator1")))

(fn ConstructionScript)