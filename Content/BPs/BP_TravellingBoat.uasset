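; Travelling boat Blueprint that provides helpers for smoothly rotating scene objects in world space.
; Three matching functions cover vertical, horizontal and circular rotation, each keeping its own stored target rotation.
; Each uses two-stage smoothing: the stored target moves at constant speed toward the requested rotation, and the object eases after it.
; The event graph and construction script are empty, so nothing in this Blueprint calls these functions.
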(event EventBeginPlay)

(event Collision|EventActorBeginOverlap
  (params (OtherActor :type Actor%20Object%20Reference)))

(event EventTick
  (params (DeltaSeconds :type Float%20%28single-precision%29)))

(fn ConstructionScript)

(fn InterpVerticalRotation
  (params (Target :type Rotator) (ConstSpeed :type Float%20%28single-precision%29) (SmoothSpeed :type Float%20%28single-precision%29) (ObjectToRotate :type Scene%20Component%20Object%20Reference))
  (bind _returnvalue (Utilities|Time|GetWorldDeltaSeconds))
  (bind _output_get (Variables|Default|SetTargetVerticalRotation (Class|KismetMathLibrary|RInterptoConstant (Variables|Default|GetTargetVerticalRotation) Target _returnvalue ConstSpeed)))
  (Transformation|SetWorldRotation ObjectToRotate (Math|Interpolation|RInterpTo (Transformation|GetWorldRotation ObjectToRotate) _output_get _returnvalue SmoothSpeed) false false))

(fn InterpHorizontalRotation
  (params (Target :type Rotator) (ConstSpeed :type Float%20%28single-precision%29) (SmoothSpeed :type Float%20%28single-precision%29) (Object :type Scene%20Component%20Object%20Reference))
  (bind _returnvalue (Utilities|Time|GetWorldDeltaSeconds))
  (bind _output_get (Variables|Default|SetTargetHorizontalRotation (Class|KismetMathLibrary|RInterptoConstant (Variables|Default|GetTargetHorizontalRotation) Target _returnvalue ConstSpeed)))
  (Transformation|SetWorldRotation Object (Math|Interpolation|RInterpTo (Transformation|GetWorldRotation Object) _output_get _returnvalue SmoothSpeed) false false))

(fn InterpCircularRotation
  (params (Target :type Rotator) (ConstSpeed :type Float%20%28single-precision%29) (SmoothSpeed :type Float%20%28single-precision%29) (Object :type Scene%20Component%20Object%20Reference))
  (bind _returnvalue (Utilities|Time|GetWorldDeltaSeconds))
  (bind _output_get (Variables|Default|SetTargetCircularRotation (Class|KismetMathLibrary|RInterptoConstant (Variables|Default|GetTargetCircularRotation) Target _returnvalue ConstSpeed)))
  (Transformation|SetWorldRotation Object (Math|Interpolation|RInterpTo (Transformation|GetWorldRotation Object) _output_get _returnvalue SmoothSpeed) false false))