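; BP_GrappleHook is a grapple hook Blueprint that records where it hits for the player's grapple.
; On Hit, it casts player 0 to BP_Player and writes the GrappleBow's world position and the hit location into the player's grapple variables.
; It then checks the distance between those points against a maximum range, but being in range only prints the target location; no pull is applied here.
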(event EventBeginPlay)

(event Collision|EventHit
  (params (MyComp :type Primitive%20Component%20Object%20Reference) (Other :type Actor%20Object%20Reference) (OtherComp :type Primitive%20Component%20Object%20Reference) (bSelfMoved :type Boolean) (HitLocation :type Vector :default "0, 0, 0") (HitNormal :type Vector :default "0, 0, 0") (NormalImpulse :type Vector :default "0, 0, 0") (Hit :type Hit%20Result%20Structure%20%28by%20ref%29))
  (bind _asbp_player (Utilities|Casting|CastToBP_Player (Game|GetPlayerCharacter 0)))
  (bind _output_get (Variables|/Game/BPs/BP_BaseCharacter.BP_BaseCharacter_C|SetGrappleStartLocation _asbp_player (Transformation|GetWorldLocation (Variables|/Game/BPs/BP_BaseCharacter.BP_BaseCharacter_C|GetGrappleBow _asbp_player))))
  (bind _output_get_2 (Variables|/Game/BPs/BP_BaseCharacter.BP_BaseCharacter_C|SetGrappleLocation _asbp_player HitLocation))
  (if (<= (Math|Vector|VectorLength (- _output_get _output_get_2)) 8e+03)
    (Development|PrintString (Utilities|String|ToString(Vector) _output_get_2))))

(fn ConstructionScript)