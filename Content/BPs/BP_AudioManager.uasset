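; Audio manager that starts a randomly selected music track on BeginPlay and fades it in.
; Looping per-frame timers are meant to step volume over configurable fade times, each fade cancelling the other.
; Fade-out, not called here, has inverted completion logic, clearing its timer while volume is still above zero.
; Track selection draws from MusicArray; its debug print rolls separately, so may name another track.
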(event Custom|EaseOutVolume
  ;[0 1 0.297] Fade Out Volume
  (bind _returnvalue (Utilities|Time|SetTimerbyEvent (EventDispatchers|CreateEvent :!event Custom|DecreaseVolume) (Utilities|Time|GetWorldDeltaSeconds) true))
  (Variables|Default|SetEaseOutHandle _returnvalue)
  (Utilities|Time|ClearandInvalidateTimerbyHandle (Variables|Default|GetEaseInHandle))
  (Development|PrintString "EaseOutVolume called" false))

(event Custom|DecreaseVolume
  (bind _maintrack (Variables|Default|GetMainTrack))
  ;[0 1 0.297] Fade Out Volume
  (bind _output_get (Variables|Default|SetFadeVolume (Math|Float|Clamp(Float) (- (Variables|Default|GetFadeVolume) (Math|Float|SafeDivide (Utilities|Time|GetWorldDeltaSeconds) (Variables|Default|GetFadeOutTime))))))
  (if (Math|Float|NearlyEqual(Float) _output_get 0.0 0.005)
    (Audio|Components|Audio|SetVolumeMultiplier _maintrack 0.0 :!class /Script/Engine.AudioComponent)
    (else
      (Audio|Components|Audio|SetVolumeMultiplier _maintrack (Variables|Default|GetFadeVolume) :!class /Script/Engine.AudioComponent)
      (Utilities|Time|ClearandInvalidateTimerbyHandle (Variables|Default|GetEaseOutHandle))
      (Development|PrintString "EaseOutVolume FINISHED" false))))

(event Custom|EaseInVolume
  ;[0 0.07739 0.4271] Fade In Volume
  (bind _returnvalue (Utilities|Time|SetTimerbyEvent (EventDispatchers|CreateEvent :!event Custom|IncreaseVolume) (Utilities|Time|GetWorldDeltaSeconds) true))
  (Variables|Default|SetEaseInHandle _returnvalue)
  (Utilities|Time|ClearandInvalidateTimerbyHandle (Variables|Default|GetEaseOutHandle))
  (Development|PrintString "EaseInVolume called" false))

(event Custom|IncreaseVolume
  (bind _maintrack (Variables|Default|GetMainTrack))
  ;[0 0.07739 0.4271] Fade In Volume
  (bind _output_get (Variables|Default|SetFadeVolume (Math|Float|Clamp(Float) (+ (Variables|Default|GetFadeVolume) (Math|Float|SafeDivide (Utilities|Time|GetWorldDeltaSeconds) (Variables|Default|GetFadeInTime))))))
  (if (< _output_get (Variables|Default|GetMainTrackVolume))
    (Audio|Components|Audio|SetVolumeMultiplier _maintrack (Variables|Default|GetFadeVolume) :!class /Script/Engine.AudioComponent)
    (else
      (Audio|Components|Audio|SetVolumeMultiplier _maintrack (Variables|Default|GetMainTrackVolume) :!class /Script/Engine.AudioComponent)
      (Utilities|Time|ClearandInvalidateTimerbyHandle (Variables|Default|GetEaseInHandle))
      (Development|PrintString "EaseInVolume FINISHED" false))))

(event EventBeginPlay
  (bind _maintrack (Variables|Default|GetMainTrack))
  (Audio|Components|Audio|SetSound _maintrack (CallFunction|SelectRandomTrack))
  (Components|Activation|Activate _maintrack true)
  (CallFunction|EaseinVolume)
  (bind _returnvalue (Game|GetCurrentLevelName true))
  (if (Utilities|Enum|Equal(Enum) _returnvalue "IntroLevel")
    (Development|PrintString "Audio mapped for Intro Level" false)))

(fn ConstructionScript)

(fn SelectRandomTrack
  (bind _musicarray (Variables|Default|GetMusicArray))
  (bind _returnvalue (Utilities|Array|Length _musicarray))
  (bind _returnvalue_2 (- _returnvalue 1))
  (bind _returnvalue_3 (Math|Random|RandomIntegerinRange 0 _returnvalue_2))
  (bind _output (Utilities|Array|Get(acopy) _musicarray _returnvalue_3))
  (Development|PrintString (Utilities|String|Append "Track: " (Utilities|GetDisplayName _output)) false)
  (return _output))