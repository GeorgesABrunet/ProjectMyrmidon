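; BP_SplinePipes is a spline-driven prop that builds bendable metal/plastic or glass pipes.
; Its construction script creates dynamic metal and glass materials, then applies exposed look settings such as age, tint, roughness and glass refraction.
; It adds a collidable spline mesh between each pair of spline points, choosing mesh by Diameter and Material, with a configurable spline up direction.
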(fn ConstructionScript
  (bind _spline (Variables|Default|GetSpline))
  (bind _material (Variables|GeneralSettings|GetMaterial))
  ;[1 1 1] Create Dynamic Material Instances
  (bind _returnvalue (Rendering|Material|CreateDynamicMaterialInstance "/Game/PluginAssets/SteampunkPropsPack/Materials/M_MetalMaster.M_MetalMaster" "None" "None" :!class /Script/Engine.KismetMaterialLibrary))
  (bind _output_get (Variables|Default|SetDynCopperMat _returnvalue))
  (bind _returnvalue_2 (Rendering|Material|CreateDynamicMaterialInstance "/Game/PluginAssets/SteampunkPropsPack/Materials/M_GlassTubeSpline_Inst.M_GlassTubeSpline_Inst" "None" "None" :!class /Script/Engine.KismetMaterialLibrary))
  (bind _output_get_2 (Variables|Default|SetDynGlassMat _returnvalue_2))
  ;[1 1 1] Apply material settings from variables.
  (Rendering|Material|SetScalarParameterValue _output_get_2 "Specular" (Variables|Appearance|GetSpecular) :!class /Script/Engine.MaterialInstanceDynamic)
  (Rendering|Material|SetScalarParameterValue _output_get_2 "Metallic" (Variables|Appearance|GetMetallic) :!class /Script/Engine.MaterialInstanceDynamic)
  (Rendering|Material|SetScalarParameterValue _output_get_2 "Normalmapstrength" (Variables|Appearance|GetNormalMapStrength) :!class /Script/Engine.MaterialInstanceDynamic)
  (Rendering|Material|SetScalarParameterValue _output_get "FadeOutTexture" (Variables|Appearance|GetFadeOutTexture) :!class /Script/Engine.MaterialInstanceDynamic)
  (Rendering|Material|SetScalarParameterValue _output_get_2 "OpacityMultiplier" (Variables|Appearance|GetOpacityMultiplier) :!class /Script/Engine.MaterialInstanceDynamic)
  (Rendering|Material|SetScalarParameterValue _output_get_2 "ReflactiveIndex" (Variables|Appearance|GetGlassRefraction) :!class /Script/Engine.MaterialInstanceDynamic)
  (Rendering|Material|SetScalarParameterValue _output_get "New-Old" (Variables|Appearance|GetAge) :!class /Script/Engine.MaterialInstanceDynamic)
  (Rendering|Material|SetScalarParameterValue _output_get "Roughness" (Variables|Appearance|GetRoughness) :!class /Script/Engine.MaterialInstanceDynamic)
  (Rendering|Material|SetScalarParameterValue (Variables|Default|GetDynCopperMat) "DesaturateTexture" (Variables|Appearance|GetDesaturateTexture) :!class /Script/Engine.MaterialInstanceDynamic)
  (Rendering|Material|SetVectorParameterValue (Variables|Default|GetDynCopperMat) "Tint" (Variables|Appearance|GetTintColor) :!class /Script/Engine.MaterialInstanceDynamic)
  ;[1 1 1] Create the Spline Meshes for each node of the spline, and apply the Spline Up Direction
  (for _index (range 0 (- (Spline|GetNumberOfSplinePoints _spline) 2))
    (bind _returnvalue_3 (AddComponent|AddSplineMeshComponent true))
    (Components|StaticMesh|SetStaticMesh _returnvalue_3 (Utilities|Select :Index (Variables|GeneralSettings|GetDiameter) :Option%200 0 :Option%201 (Utilities|Select :Index _material :NewEnumerator0 "/Game/PluginAssets/SteampunkPropsPack/Meshes/SplineMeshes/SplinePipeSegment1.SplinePipeSegment1" :NewEnumerator1 "/Game/PluginAssets/SteampunkPropsPack/Meshes/SplineMeshes/GlassTubeSplineMesh01.GlassTubeSplineMesh01") :Option%202 (Utilities|Select :Index _material :NewEnumerator0 "/Game/PluginAssets/SteampunkPropsPack/Meshes/SplineMeshes/SplinePipeSegment2.SplinePipeSegment2" :NewEnumerator1 "/Game/PluginAssets/SteampunkPropsPack/Meshes/SplineMeshes/GlassTubeSplineMesh02.GlassTubeSplineMesh02") :Option%203 (Utilities|Select :Index _material :NewEnumerator0 "/Game/PluginAssets/SteampunkPropsPack/Meshes/SplineMeshes/SplinePipeSegment3.SplinePipeSegment3" :NewEnumerator1 "/Game/PluginAssets/SteampunkPropsPack/Meshes/SplineMeshes/GlassTubeSplineMesh03.GlassTubeSplineMesh03") :Option%204 (Utilities|Select :Index _material :NewEnumerator0 "/Game/PluginAssets/SteampunkPropsPack/Meshes/SplineMeshes/SplinePipeSegment4.SplinePipeSegment4" :NewEnumerator1 "/Game/PluginAssets/SteampunkPropsPack/Meshes/SplineMeshes/GlassTubeSplineMesh04.GlassTubeSplineMesh04")))
    (Rendering|Material|SetMaterial _returnvalue_3 0 (Utilities|Select :Index (Variables|GeneralSettings|GetMaterial) :NewEnumerator0 (Variables|Default|GetDynCopperMat) :NewEnumerator1 (Variables|Default|GetDynGlassMat)))
    (Collision|SetCollisionEnabled _returnvalue_3 "QueryAndPhysics")
    (Transformation|AttachComponentToComponent _returnvalue_3 (Variables|Default|GetSceneRoot) "None" "KeepRelative" "KeepRelative" "KeepRelative" true)
    (SplineMesh|SetStartandEnd _returnvalue_3 (.Location (Spline|GetLocationandTangentatSplinePoint _spline _index "Local")) (.Tangent (Spline|GetLocationandTangentatSplinePoint _spline _index "Local")) (.Location (Spline|GetLocationandTangentatSplinePoint _spline (+ _index 1) "Local")) (.Tangent (Spline|GetLocationandTangentatSplinePoint _spline (+ _index 1) "Local")) true :!class /Script/Engine.SplineMeshComponent)
    (SplineMesh|SetSplineUpDir _returnvalue_3 (Variables|GeneralSettings|GetSplineUpDir) true)))