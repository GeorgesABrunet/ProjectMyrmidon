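; Steampunk compass prop whose needle can spin, rest at a set rotation, or point at the BP_CompassTarget with a matching index.
; Construction Script sets tilt, socket fittings, initial needle angle and dynamic materials for face, aging and tint.
; Tick derives target bearing via atan2 minus actor yaw, feeding the needle directly or as the base for timeline-driven wobble.
; Optional demo mode animates material age and roughness for the example map.
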(event Custom|EventStopSpin
  ;[1 1 1] Start and Stop Needle Spinning(This can be triggered at runtime)
  (bind _spin (Timeline|SpinTimeline Stop)
    (:Update
      (Transformation|SetRelativeRotation (Variables|Default|GetGaugeNeedle) (Math|Rotator|MakeRotator (* _spin 3.6e+02) 0.0 0.0) false false))))

(event Custom|EventSetTarget
  ;[1 1 1] Get All Instances of Compass Target in the level and select the once with matching Index
  (bind _outactors (Actor|GetAllActorsOfClass "/Game/PluginAssets/SteampunkPropsPack/Blueprints/BP_CompassTarget.BP_CompassTarget_C"))
  (for _array_element _outactors
    (if (== (Variables|/Game/PluginAssets/SteampunkPropsPack/Blueprints/BP_CompassTarget.BP_CompassTarget_C|GetIndex _array_element) (Variables|GeneralSettings|GetTargetIndex))
      (Variables|Default|SetTargetObjectReference _array_element))))

(event Custom|EventStartSpin
  ;[1 1 1] Start and Stop Needle Spinning(This can be triggered at runtime)
  (Components|Timeline|SetPlayRate (Variables|Default|GetSpinTimeline) (Variables|Spin|GetRotationSpeed))
  (bind _spin (Timeline|SpinTimeline Play)
    (:Update
      (Transformation|SetRelativeRotation (Variables|Default|GetGaugeNeedle) (Math|Rotator|MakeRotator (* _spin 3.6e+02) 0.0 0.0) false false))))

(event Custom|EventStartRandomNeedleMovement
  ;[1 1 1] Make the needle move randomly for a more natural look
  (Components|Timeline|SetPlayRate (Variables|Default|GetRandomMovementTimeline) 0.5)
  (bind _needlemovement (Timeline|RandomMovementTimeline Play)
    (:Update
      (Variables|Default|SetNeedlePositionCache (+ (* _needlemovement (Variables|GeneralSettings|GetNeedleRandomMovement)) (Variables|GeneralSettings|GetNeedleRotation)))
      (CallFunction|EventUpdateNeedle))))

(event Custom|EventUpdateNeedle
  ;[1 1 1] Update the desired needle position
  (Transformation|SetRelativeRotation (Variables|Default|GetGaugeNeedle) (Math|Rotator|MakeRotator (Math|Float|MapRangeUnclamped (Variables|Default|GetNeedlePositionCache) 0.0 1.0 0.0 3.6e+02) 0.0 0.0) false false))

(event Custom|EventDemo
  (bind _dynglassmat (Variables|Default|GetDynGlassMat))
  ;[1 1 1] This is the Demo Mode that is used in the Example map. It can Be removed if desired.
  (Components|Timeline|SetPlayRate (Variables|Default|GetAgeTimeline) 0.5)
  (bind (_direction _age _roughness_) (Timeline|AgeTimeline Play)
    (:Update
      (Rendering|Material|SetScalarParameterValue _dynglassmat "New-Old" _age :!class /Script/Engine.MaterialInstanceDynamic)
      (Rendering|Material|SetScalarParameterValue _dynglassmat "Roughness" _roughness_ :!class /Script/Engine.MaterialInstanceDynamic))))

(event EventBeginPlay
  (CallFunction|EventSetTarget)
  ;[1 1 1] Start Random Needle Movement if NeedleRandomMovement>0
  (if (> (Variables|GeneralSettings|GetNeedleRandomMovement) 0.0)
    (CallFunction|EventStartRandomNeedleMovement))
  ;[1 1 1] Check SpinOnBeginPlay and DemoMode, and trigger the events
  (if (Variables|Spin|GetSpinOnBeginPlay)
    (CallFunction|EventStartSpin))
  ;;[1 1 1] You can remove this if you do not need Demo Mode
  (if (Variables|Default|GetDemoMode)
    (CallFunction|EventDemo)))

(event EventTick
  (params (DeltaSeconds :type Float%20%28single-precision%29))
  (bind _returnvalue (Transformation|GetActorLocation))
  (bind _returnvalue_2 (Transformation|GetActorRotation))
  (bind _targetobjectreference (Variables|Default|GetTargetObjectReference))
  (bind _yaw (Math|Rotator|BreakRotator _returnvalue_2))
  (bind _returnvalue_3 (Transformation|GetActorLocation _targetobjectreference))
  (bind _returnvalue_4 (- _returnvalue_3 _returnvalue))
  (bind (_x _y) (Math|Vector|BreakVector _returnvalue_4))
  (bind _returnvalue_5 (Class|KismetMathLibrary|DegAtan2 _y _x))
  (bind _returnvalue_6 (- _returnvalue_5 _yaw))
  (bind _returnvalue_7 (> _returnvalue_6 0.0))
  (bind _returnvalue_8 (+ _returnvalue_6 3.6e+02))
  (bind _returnvalue_9 (select _returnvalue_7 _returnvalue_6 _returnvalue_8))
  (bind _returnvalue_10 (Math|Float|MapRangeClamped _returnvalue_9 0.0 3.6e+02 0.0 1.0))
  ;[1 1 1] Make the Needle point to the Target if PointToTarget is ticked
  (if (Utilities|IsValid _targetobjectreference)
    (if (Variables|GeneralSettings|GetPointToTarget)
      (if (> (Variables|GeneralSettings|GetNeedleRandomMovement) 0.0)
        (Variables|GeneralSettings|SetNeedleRotation _returnvalue_10)
        (else
          (Variables|Default|SetNeedlePositionCache _returnvalue_10)
          (CallFunction|EventUpdateNeedle))))))

(fn ConstructionScript
  (bind _rightsocket (Variables|Default|GetRightSocket))
  (bind _topsocket (Variables|Default|GetTopSocket))
  (bind _socketdiameter (Variables|GeneralSettings|GetSocketDiameter))
  (bind _gaugemesh (Variables|Default|GetGaugeMesh))
  (bind _facevariation (Variables|GeneralSettings|GetFaceVariation))
  (bind _socketlength (Variables|GeneralSettings|GetSocketLength))
  (bind _returnvalue (Math|Float|MapRangeClamped _socketlength 0.5 2.0 9.0 9.8))
  (bind _returnvalue_2 (* _returnvalue -1.0))
  ;[1 1 1] Get All Instances of Compass Target in the level and select the once with matching Index
  (bind _outactors (Actor|GetAllActorsOfClass "/Game/PluginAssets/SteampunkPropsPack/Blueprints/BP_CompassTarget.BP_CompassTarget_C"))
  (for _array_element _outactors
    (if (== (Variables|/Game/PluginAssets/SteampunkPropsPack/Blueprints/BP_CompassTarget.BP_CompassTarget_C|GetIndex _array_element) (Variables|GeneralSettings|GetTargetIndex))
      (Variables|Default|SetTargetObjectReference _array_element)))
  ;[1 1 1] Adjust the Tilt of the Compass
  (Transformation|SetRelativeRotation (Variables|Default|GetGaugeMesh) (Math|Rotator|MakeRotator 0.0 (Math|Float|MapRangeClamped (Variables|GeneralSettings|GetCompassTilt) -1.0 1.0 9e+01 -9e+01) 0.0) false false)
  ;[1 1 1] Make the Needle point to the Target if PointToTarget is ticked
  (if (and (Variables|GeneralSettings|GetPointToTarget) (Utilities|IsValid (Variables|Default|GetTargetObjectReference)))
    (Transformation|SetRelativeRotation (Variables|Default|GetGaugeNeedle) (Math|Rotator|MakeRotator (- (Class|KismetMathLibrary|DegAtan2 (.Y (Math|Vector|BreakVector (- (Transformation|GetActorLocation (Variables|Default|GetTargetObjectReference)) (Transformation|GetActorLocation)))) (.X (Math|Vector|BreakVector (- (Transformation|GetActorLocation (Variables|Default|GetTargetObjectReference)) (Transformation|GetActorLocation))))) (.Yaw (Math|Rotator|BreakRotator (Transformation|GetActorRotation)))) 0.0 0.0) false false))
  ;[1 1 1] Create Dynamic Material Instances
  (bind _returnvalue_3 (Rendering|Material|CreateDynamicMaterialInstance "/Game/PluginAssets/SteampunkPropsPack/Materials/M_GaugeFaces.M_GaugeFaces" "None" "None" :!class /Script/Engine.KismetMaterialLibrary))
  (bind _output_get (Variables|Default|SetDynMatFace _returnvalue_3))
  (bind _returnvalue_4 (Rendering|Material|CreateDynamicMaterialInstance "/Game/PluginAssets/SteampunkPropsPack/Materials/M_GaugeGlass_Inst.M_GaugeGlass_Inst" "None" "None" :!class /Script/Engine.KismetMaterialLibrary))
  (bind _output_get_2 (Variables|Default|SetDynGlassMat _returnvalue_4))
  (bind _returnvalue_5 (Rendering|Material|CreateDynamicMaterialInstance "/Game/PluginAssets/SteampunkPropsPack/Materials/M_MetalMaster.M_MetalMaster" "None" "None" :!class /Script/Engine.KismetMaterialLibrary))
  (bind _output_get_3 (Variables|Default|SetDynMetalMat _returnvalue_5))
  ;[1 1 1] Set Material Settings
  (Rendering|Material|SetScalarParameterValue _output_get_3 "FadeOutTexture" (Variables|Appearance|GetFadeOutTexture) :!class /Script/Engine.MaterialInstanceDynamic)
  (Rendering|Material|SetScalarParameterValue _output_get_3 "Specular" (Variables|Appearance|GetSpecular) :!class /Script/Engine.MaterialInstanceDynamic)
  (Rendering|Material|SetScalarParameterValue _output_get_3 "Metallic" (Variables|Appearance|GetMetallic) :!class /Script/Engine.MaterialInstanceDynamic)
  (Rendering|Material|SetScalarParameterValue _output_get_3 "New-Old" (Variables|Appearance|GetAgeMetal) :!class /Script/Engine.MaterialInstanceDynamic)
  (Rendering|Material|SetScalarParameterValue _output_get_3 "Roughness" (Variables|Appearance|GetRoughness) :!class /Script/Engine.MaterialInstanceDynamic)
  (Rendering|Material|SetScalarParameterValue _output_get_3 "DesaturateTexture" (Variables|Appearance|GetDesaturateMetal) :!class /Script/Engine.MaterialInstanceDynamic)
  (Rendering|Material|SetScalarParameterValue _output_get_3 "NormalMapStrength" (Variables|Appearance|GetNormalMapStrength) :!class /Script/Engine.MaterialInstanceDynamic)
  (Rendering|Material|SetScalarParameterValue (Variables|Default|GetDynGlassMat) "New-Old" (Variables|Appearance|GetAgeGlass) :!class /Script/Engine.MaterialInstanceDynamic)
  (Rendering|Material|SetVectorParameterValue _output_get_3 "Tint" (Variables|Appearance|GetMetalTintColor) :!class /Script/Engine.MaterialInstanceDynamic)
  (Rendering|Material|SetVectorParameterValue (Variables|Default|GetDynMatFace) "Tint" (Variables|Appearance|GetFaceTintColor) :!class /Script/Engine.MaterialInstanceDynamic)
  (Rendering|Material|SetScalarParameterValue (Variables|Default|GetDynMatFace) "DesaturateTexture" (Variables|Appearance|GetDesaturateFace) :!class /Script/Engine.MaterialInstanceDynamic)
  (Rendering|Material|SetTextureParameterValue (Variables|Default|GetDynMatFace) "DiffuseNew" (Utilities|Select :Index _facevariation :Option%200 0 :Option%201 "/Game/PluginAssets/SteampunkPropsPack/Textures/T_GaugeFace02New_D.T_GaugeFace02New_D" :Option%202 "/Game/PluginAssets/SteampunkPropsPack/Textures/T_GaugeFace04New_D.T_GaugeFace04New_D"))
  (Rendering|Material|SetTextureParameterValue (Variables|Default|GetDynMatFace) "DiffuseOld" (Utilities|Select :Index _facevariation :Option%200 0 :Option%201 "/Game/PluginAssets/SteampunkPropsPack/Textures/T_GaugeFace02Old_D.T_GaugeFace02Old_D" :Option%202 "/Game/PluginAssets/SteampunkPropsPack/Textures/T_GaugeFace04Old_D.T_GaugeFace04Old_D"))
  ;[1 1 1] Apply Materials to Mesh
  (Rendering|Material|SetMaterial _gaugemesh 0 (Variables|Default|GetDynGlassMat))
  (Rendering|Material|SetMaterial _gaugemesh 1 (Variables|Default|GetDynMetalMat))
  (Rendering|Material|SetMaterial _gaugemesh 2 (Variables|Default|GetDynMatFace))
  (Rendering|Material|SetMaterial _gaugemesh 3 (Variables|Default|GetDynMetalMat))
  ;[1 1 1] Set Needle Rotation if Point to Target is not ticked
  (Variables|Default|SetNeedlePositionCache (Variables|GeneralSettings|GetNeedleRotation))
  (if (Variables|GeneralSettings|GetPointToTarget)
    _
    (else
      (Transformation|SetRelativeRotation (Variables|Default|GetGaugeNeedle) (Math|Rotator|MakeRotator (Math|Float|MapRangeClamped (Variables|Default|GetNeedlePositionCache) 0.0 1.0 0.0 3.6e+02) 0.0 0.0) false false)))
  ;[1 1 1] Set Socket Settings
  (Rendering|Material|SetMaterial _topsocket 0 (Variables|Default|GetDynMetalMat))
  (Transformation|SetRelativeScale3D _rightsocket (Math|Vector|MakeVector _socketdiameter _socketdiameter _socketlength))
  (Transformation|SetRelativeLocation _topsocket (Math|Vector|MakeVector 0.0 0.0 _returnvalue) false false)
  (Transformation|SetRelativeLocation (Variables|Default|GetBottomSocket) (Math|Vector|MakeVector 0.0 0.0 _returnvalue_2) false false)
  (Transformation|SetRelativeLocation _rightsocket (Math|Vector|MakeVector 0.0 _returnvalue 0.0) false false)
  (Transformation|SetRelativeLocation (Variables|Default|GetLeftSocket) (Math|Vector|MakeVector 0.0 _returnvalue_2 0.0) false false)
  ;[1 1 1] Add Sockets
  (Rendering|SetVisibility (Variables|Default|GetTopSocket) (Variables|GeneralSettings|GetAddTopSocket) false)
  (Rendering|SetVisibility (Variables|Default|GetRightSocket) (Variables|GeneralSettings|GetAddRightSocket) false)
  (Rendering|SetVisibility (Variables|Default|GetBottomSocket) (Variables|GeneralSettings|GetAddBottonSocket) false)
  (Rendering|SetVisibility (Variables|Default|GetLeftSocket) (Variables|GeneralSettings|GetAddLeftSocket) false))