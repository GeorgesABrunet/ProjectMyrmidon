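; BP_Gear is a configurable steampunk gear prop that can spin at runtime or on BeginPlay.
; The construction script picks the gear mesh variant and optional sized pin, then applies one dynamic metal material with exposed wear, surface and tint settings to both.
; A timeline drives yaw rotation at RotationSpeed through start and stop events.
; An optional demo mode animates age and roughness for the example map.
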(event Custom|EventStopSpin
  ;[1 1 1] Start and Stop Gear Spinning(This can be triggered at runtime)
  (bind _spin (Timeline|SpinTimeline Stop)
    (:Update
      (Transformation|SetRelativeRotation (Variables|Default|GetGearMesh) (Math|Rotator|MakeRotator 0.0 0.0 (* _spin 3.6e+02)) false false))))

(event Custom|EventStartSpin
  ;[1 1 1] Start and Stop Gear Spinning(This can be triggered at runtime)
  (Components|Timeline|SetPlayRate (Variables|Default|GetSpinTimeline) (Variables|Spin|GetRotationSpeed))
  (bind _spin (Timeline|SpinTimeline Play)
    (:Update
      (Transformation|SetRelativeRotation (Variables|Default|GetGearMesh) (Math|Rotator|MakeRotator 0.0 0.0 (* _spin 3.6e+02)) false false))))

(event Custom|EventDemo
  (bind _dynmat01 (Variables|Default|GetDynMat01))
  ;[1 1 1] This is the Demo Mode that is used in the Example map. It can Be removed if desired.
  (Components|Timeline|SetPlayRate (Variables|Default|GetAgeTimeline) 0.5)
  (bind (_direction _age _roughness_) (Timeline|AgeTimeline Play)
    (:Update
      (Rendering|Material|SetScalarParameterValue _dynmat01 "New-Old" _age :!class /Script/Engine.MaterialInstanceDynamic)
      (Rendering|Material|SetScalarParameterValue _dynmat01 "Roughness" _roughness_ :!class /Script/Engine.MaterialInstanceDynamic))))

(event EventBeginPlay
  ;[1 1 1] Check if Gear should start spinning on Begin Play
  (if (Variables|Spin|GetSpinOnBeginPlay)
    (CallFunction|EventStartSpin))
  ;;[1 1 1] You can remove this if you do not need Demo Mode
  (if (Variables|Default|GetDemoMode)
    (CallFunction|EventDemo)))

(fn ConstructionScript
  (bind _gearpin01 (Variables|Default|GetGearPin01))
  ;[1 1 1] Setup the Gear Variation and Pin
  (Rendering|SetVisibility _gearpin01 (Variables|GeneralSettings|GetAddPin) false)
  (Transformation|SetRelativeScale3D _gearpin01 (Utilities|Select :Index (Variables|GeneralSettings|GetPinSize) :Option%200 "1.000000,1.000000,1.000000" :Option%201 "0.300000,0.300000,1.500000" :Option%202 "0.500000,0.500000,1.500000" :Option%203 "1.000000,1.000000,1.100000" :Option%204 "1.500000,1.500000,1.500000"))
  (Components|StaticMesh|SetStaticMesh (Variables|Default|GetGearMesh) (Utilities|Select :Index (Variables|GeneralSettings|GetGearVariation) :Option%200 0 :Option%201 "/Game/PluginAssets/SteampunkPropsPack/Meshes/SM_Gear01.SM_Gear01" :Option%202 "/Game/PluginAssets/SteampunkPropsPack/Meshes/SM_Gear02.SM_Gear02" :Option%203 "/Game/PluginAssets/SteampunkPropsPack/Meshes/SM_Gear03.SM_Gear03" :Option%204 "/Game/PluginAssets/SteampunkPropsPack/Meshes/SM_Gear04.SM_Gear04" :Option%205 "/Game/PluginAssets/SteampunkPropsPack/Meshes/SM_Gear05.SM_Gear05" :Option%206 "/Game/PluginAssets/SteampunkPropsPack/Meshes/SM_Gear06.SM_Gear06"))
  ;[1 1 1] Create Dynamic Material Instance
  (bind _returnvalue (Rendering|Material|CreateDynamicMaterialInstance "/Game/PluginAssets/SteampunkPropsPack/Materials/M_MetalGears_Inst.M_MetalGears_Inst" "None" "None" :!class /Script/Engine.KismetMaterialLibrary))
  (bind _output_get (Variables|Default|SetDynMat01 _returnvalue))
  ;[1 1 1] Apply the variable values to the Dynamic Material
  (Rendering|Material|SetScalarParameterValue _output_get "FadeOutTexture" (Variables|Appearance|GetFadeOutTexture) :!class /Script/Engine.MaterialInstanceDynamic)
  (Rendering|Material|SetScalarParameterValue _output_get "Specular" (Variables|Appearance|GetSpecular) :!class /Script/Engine.MaterialInstanceDynamic)
  (Rendering|Material|SetScalarParameterValue _output_get "Metallic" (Variables|Appearance|GetMetallic) :!class /Script/Engine.MaterialInstanceDynamic)
  (Rendering|Material|SetScalarParameterValue _output_get "New-Old" (Variables|Appearance|GetAge) :!class /Script/Engine.MaterialInstanceDynamic)
  (Rendering|Material|SetScalarParameterValue _output_get "Roughness" (Variables|Appearance|GetRoughness) :!class /Script/Engine.MaterialInstanceDynamic)
  (Rendering|Material|SetScalarParameterValue _output_get "DesaturateTexture" (Variables|Appearance|GetDesaturateTexture) :!class /Script/Engine.MaterialInstanceDynamic)
  (Rendering|Material|SetScalarParameterValue _output_get "NormalMapStrength" (Variables|Appearance|GetNormalMapStrength) :!class /Script/Engine.MaterialInstanceDynamic)
  (Rendering|Material|SetVectorParameterValue _output_get "Tint" (Variables|Appearance|GetTintColor) :!class /Script/Engine.MaterialInstanceDynamic)
  ;[1 1 1] Apply Material to Static Meshes
  (Rendering|Material|SetMaterial (Variables|Default|GetGearMesh) 0 _output_get))