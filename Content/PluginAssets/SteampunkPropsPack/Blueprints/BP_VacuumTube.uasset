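; Configurable steampunk vacuum tube prop with selectable tube, socket and shield meshes, a pulsing plate glow and optional spin.
; The construction script sets mesh variations, hiding any set to zero, and builds dynamic glow, glass, metal and two-sided materials from user settings.
; On BeginPlay, a timeline drives emissive glow using two curves or Tick-refreshed random values.
; Another timeline rotates the tube, startable on play or at runtime.
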(event Custom|EventStopSpin
  ;[1 1 1] Start and Stop Tube Spinning(This can be triggered at runtime)
  (bind _spin (Timeline|SpinTimeline Stop)
    (:Update
      (Transformation|AddLocalRotation (Variables|Default|GetTubeMesh) (Math|Rotator|MakeRotator 0.0 0.0 (* _spin (Variables|Spin|GetRotationSpeed))) false false))))

(event Custom|EventStartSpin
  ;[1 1 1] Start and Stop Tube Spinning(This can be triggered at runtime)
  (bind _spin (Timeline|SpinTimeline Play)
    (:Update
      (Transformation|AddLocalRotation (Variables|Default|GetTubeMesh) (Math|Rotator|MakeRotator 0.0 0.0 (* _spin (Variables|Spin|GetRotationSpeed))) false false))))

(event Custom|EventApplyGlowSettings
  ;[1 1 1] Apply the Glow Settings
  (Rendering|Material|SetScalarParameterValue (Variables|Default|GetDynGlowMat) "EmissiveMultiplier" (Variables|Glow|GetTubeGlowConstant) :!class /Script/Engine.MaterialInstanceDynamic)
  (Components|Timeline|SetPlayRate (Variables|Default|GetGlowTimeline) (Variables|Glow|GetPulseFrequency)))

(event EventBeginPlay
  (bind _tubeglowmin (Variables|Glow|GetTubeGlowMin))
  (Utilities|FlowControl|Sequence
    (:then_0
      ;[1 1 1] Check if Winder should start spinning on Begin Play
      (if (Variables|Spin|GetSpinOnBeginPlay)
        (CallFunction|EventStartSpin)))
    (:then_1
      ;[1 1 1] Pulse the glow of the Tube Plates according to PulseType
      (if (Variables|Glow|GetPulseGlow)
        (Utilities|FlowControl|Sequence
          (:then_0
            (bind (_direction _pulse01 _pulse02) (Timeline|GlowTimeline SetNewTime)
              (:Update
                (Variables|Glow|SetTubeGlowConstant (+ (* (Utilities|Select :Index (Variables|Glow|GetPulseType) :NewEnumerator0 _pulse01 :NewEnumerator1 _pulse02 :NewEnumerator2 (Variables|Default|GetRandomPulse)) (- (Variables|Glow|GetTubeGlowMax) _tubeglowmin)) _tubeglowmin))
                (CallFunction|EventApplyGlowSettings))))
          (:then_1
            (Timeline|GlowTimeline Play)))))))

(event EventTick
  (params (DeltaSeconds :type Float%20%28single-precision%29))
  ;[1 1 1] Set Random values for pulse if PulseType is set to Random
  (if (Utilities|Enum|Equal(Enum) (Variables|Glow|GetPulseType) "NewEnumerator2")
    (Utilities|FlowControl|Delay (/ 0.1 (Variables|Glow|GetPulseFrequency)))
    (Variables|Default|SetRandomPulse (Math|Random|RandomFloatinRange 0.0 1.0))))

(fn ConstructionScript
  (bind _shieldvariation (Variables|GeneralSettings|GetShieldVariation))
  (bind _socketvariation (Variables|GeneralSettings|GetSocketVariation))
  (bind _socketmesh (Variables|Default|GetSocketMesh))
  (bind _tubeshieldmesh (Variables|Default|GetTubeShieldMesh))
  (bind _tubemesh (Variables|Default|GetTubeMesh))
  (bind _tubemesh_2 (Variables|Default|GetTubeMesh))
  (bind _tubevariation (Variables|GeneralSettings|GetTubeVariation))
  ;[1 1 1] Setup Variations
  (Components|StaticMesh|SetStaticMesh _tubemesh (Utilities|Select :Index _tubevariation :Option%200 "/Game/PluginAssets/SteampunkPropsPack/Meshes/SM_VacuumTube01.SM_VacuumTube01" :Option%201 "/Game/PluginAssets/SteampunkPropsPack/Meshes/SM_VacuumTube01.SM_VacuumTube01" :Option%202 "/Game/PluginAssets/SteampunkPropsPack/Meshes/SM_VacuumTube02.SM_VacuumTube02" :Option%203 "/Game/PluginAssets/SteampunkPropsPack/Meshes/SM_VacuumTube03.SM_VacuumTube03" :Option%204 "/Game/PluginAssets/SteampunkPropsPack/Meshes/SM_VacuumTube04.SM_VacuumTube04"))
  (Components|StaticMesh|SetStaticMesh _socketmesh (Utilities|Select :Index _socketvariation :Option%200 "/Game/PluginAssets/SteampunkPropsPack/Meshes/SM_Socket01.SM_Socket01" :Option%201 "/Game/PluginAssets/SteampunkPropsPack/Meshes/SM_Socket01.SM_Socket01" :Option%202 "/Game/PluginAssets/SteampunkPropsPack/Meshes/SM_Socket02.SM_Socket02"))
  (Components|StaticMesh|SetStaticMesh _tubeshieldmesh (Utilities|Select :Index _shieldvariation :Option%200 "/Game/PluginAssets/SteampunkPropsPack/Meshes/SM_TubeShield1.SM_TubeShield1" :Option%201 "/Game/PluginAssets/SteampunkPropsPack/Meshes/SM_TubeShield1.SM_TubeShield1" :Option%202 "/Game/PluginAssets/SteampunkPropsPack/Meshes/SM_TubeShield2.SM_TubeShield2"))
  (Rendering|SetVisibility _tubemesh (> _tubevariation 0) false)
  (Rendering|SetVisibility _socketmesh (> _socketvariation 0) false)
  (Rendering|SetVisibility _tubeshieldmesh (> _shieldvariation 0) false)
  ;[1 1 1] Create and Apply Dynamic Materials and apply user settings
  (bind _returnvalue (Rendering|Material|CreateDynamicMaterialInstance "/Game/PluginAssets/SteampunkPropsPack/Materials/M_VacTubePlatesGlow_Inst.M_VacTubePlatesGlow_Inst" "None" "None" :!class /Script/Engine.KismetMaterialLibrary))
  (bind _output_get (Variables|Default|SetDynGlowMat _returnvalue))
  (Rendering|Material|SetScalarParameterValue _output_get "EmissiveMultiplier" (Variables|Glow|GetTubeGlowConstant) :!class /Script/Engine.MaterialInstanceDynamic)
  (bind _returnvalue_2 (Rendering|Material|CreateDynamicMaterialInstance "/Game/PluginAssets/SteampunkPropsPack/Materials/M_GlassMaster.M_GlassMaster" "None" "None" :!class /Script/Engine.KismetMaterialLibrary))
  (bind _output_get_2 (Variables|Default|SetDynGlassMat _returnvalue_2))
  (Rendering|Material|SetScalarParameterValue _output_get_2 "New-Old" (Variables|Appearance|GetAgeGlass) :!class /Script/Engine.MaterialInstanceDynamic)
  (Rendering|Material|SetScalarParameterValue _output_get_2 "Roughness" (Variables|Appearance|GetRoughness) :!class /Script/Engine.MaterialInstanceDynamic)
  (bind _returnvalue_3 (Rendering|Material|CreateDynamicMaterialInstance "/Game/PluginAssets/SteampunkPropsPack/Materials/M_MetalMaster.M_MetalMaster" "None" "None" :!class /Script/Engine.KismetMaterialLibrary))
  (bind _output_get_3 (Variables|Default|SetDynMetalMat _returnvalue_3))
  (bind _returnvalue_4 (Rendering|Material|CreateDynamicMaterialInstance "/Game/PluginAssets/SteampunkPropsPack/Materials/M_TwoSidedMaster.M_TwoSidedMaster" "None" "None" :!class /Script/Engine.KismetMaterialLibrary))
  (bind _output_get_4 (Variables|Default|SetDynTwoSidedMat _returnvalue_4))
  (Rendering|Material|SetScalarParameterValue _output_get_4 "New-Old" (Variables|Appearance|GetAgeGlass) :!class /Script/Engine.MaterialInstanceDynamic)
  (Rendering|Material|SetScalarParameterValue _output_get_3 "New-Old" (Variables|Appearance|GetAgeMetal) :!class /Script/Engine.MaterialInstanceDynamic)
  (Rendering|Material|SetScalarParameterValue _output_get_3 "Roughness" (Variables|Appearance|GetRoughness) :!class /Script/Engine.MaterialInstanceDynamic)
  (Rendering|Material|SetMaterial (Variables|Default|GetSocketMesh) 0 _output_get_3)
  (Rendering|Material|SetScalarParameterValue (Variables|Default|GetDynMetalMat) "Specular" (Variables|Appearance|GetSpecular) :!class /Script/Engine.MaterialInstanceDynamic)
  (Rendering|Material|SetScalarParameterValue (Variables|Default|GetDynMetalMat) "Metallic" (Variables|Appearance|GetMetallic) :!class /Script/Engine.MaterialInstanceDynamic)
  (Rendering|Material|SetScalarParameterValue (Variables|Default|GetDynMetalMat) "Normalmapstrength" (Variables|Appearance|GetNormalMapStrength) :!class /Script/Engine.MaterialInstanceDynamic)
  (Rendering|Material|SetScalarParameterValue (Variables|Default|GetDynMetalMat) "FadeOutTexture" (Variables|Appearance|GetFadeOutTexture) :!class /Script/Engine.MaterialInstanceDynamic)
  (Rendering|Material|SetScalarParameterValue (Variables|Default|GetDynGlassMat) "ReflactiveIndex" (Variables|Appearance|GetGlassRefraction) :!class /Script/Engine.MaterialInstanceDynamic)
  (Rendering|Material|SetScalarParameterValue (Variables|Default|GetDynMetalMat) "DesaturateTexture" (Variables|Appearance|GetDesaturateTexture) :!class /Script/Engine.MaterialInstanceDynamic)
  (Rendering|Material|SetVectorParameterValue (Variables|Default|GetDynMetalMat) "Tint" (Variables|Appearance|GetTintColor) :!class /Script/Engine.MaterialInstanceDynamic)
  (Rendering|Material|SetVectorParameterValue _output_get "GlowColor" (Variables|Glow|GetGlowColor) :!class /Script/Engine.MaterialInstanceDynamic)
  (Rendering|Material|SetMaterial _tubemesh_2 0 (Variables|Default|GetDynTwoSidedMat))
  (Rendering|Material|SetMaterial _tubemesh_2 1 (Variables|Default|GetDynGlassMat))
  (Rendering|Material|SetMaterial _tubemesh_2 2 (Variables|Default|GetDynMetalMat))
  (Rendering|Material|SetMaterial _tubemesh_2 3 (Variables|Default|GetDynGlowMat)))